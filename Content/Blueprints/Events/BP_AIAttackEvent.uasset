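; BP_AIAttackEvent is an AI event that makes the controlled pawn attack a target through the Gameplay Ability System.
; On begin, it caches the pawn's DP_AbilitySystemComponent and hands it the target actor.
; On each update, it tries to activate abilities matching the attack tag, leaving the attack itself to those abilities.
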(event `self.OnBeginBP`
  (bind _asdp_ability_system_component (cast `DP_AbilitySystemComponent` (`AbilitySystemBlueprintLibrary.GetAbilitySystemComponent` (`Controller.K2_GetPawn` (`self.ControllerRef`)))))
  (bind _output_get (set `self.AbilitySystemComponentRef` _asdp_ability_system_component))
  (set `DP_AbilitySystemComponent.TargetActorRef` (`self.TargetActorRef`) _output_get))

(event `self.OnUpdateBP`
  (`AbilitySystemComponent.TryActivateAbilitiesByTag` (`self.AbilitySystemComponentRef`) (`BlueprintGameplayTagLibrary.MakeGameplayTagContainerFromTag` (`self.AttackAbilityTag`)) true))