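; BP_MeeleEnemy is a melee enemy character that chases and attacks the player by pushing behavior events onto an event handler.
; StartDefaultEvent creates a chase event with its AI controller and the player's pawn as target, then pushes it to the handler.
; When a player character overlaps its sphere, it pushes an attack event on that actor.
; Any overlap end marks the stored attack event done and clears it.
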(event `self.StartDefaultEvent`
  (bind _chaseeventref (`self.ChaseEventRef`))
  (bind _returnvalue (`|GenericCreateObject` (`self.ChaseClass`)))
  (bind _output_get (set `self.ChaseEventRef` _returnvalue))
  (`DP_ChasePlayerEvent.SetEventHandler` _output_get (`self.EnemyEventHandlerRef`))
  (bind _asaicontroller (cast `AIController` (`self.GetController`)))
  (`DP_ChasePlayerEvent.SetController` (`self.ChaseEventRef`) _asaicontroller)
  (`DP_ChasePlayerEvent.SetTarget` _chaseeventref (`Controller.K2_GetPawn` (`GameplayStatics.GetPlayerController` 0)))
  (`DP_EventHandler.PushEvent` (`self.EnemyEventHandlerRef`) _chaseeventref))

(event `self.Sphere.OnComponentBeginOverlap`
  (params (OverlappedComponent :type "PrimitiveComponent Object Reference") (OtherActor :type "Actor Object Reference") (OtherComp :type "PrimitiveComponent Object Reference") (OtherBodyIndex :type Integer) (bFromSweep :type Boolean) (SweepResult :type "HitResult Structure (by ref)"))
  (bind _attackeventref (`self.AttackEventRef`))
  (if (== (`GameplayStatics.GetObjectClass` OtherActor) "/Game/Blueprints/Characters/BP_PlayerCharacter.BP_PlayerCharacter_C")
    (bind _returnvalue (`|GenericCreateObject` (`self.AttackClass`)))
    (bind _output_get (set `self.AttackEventRef` _returnvalue))
    (`DP_AIAttackEvent.SetTargetActorRef` _output_get OtherActor)
    (`DP_AIBaseEvent.SetEventHandler` _output_get (`self.EnemyEventHandlerRef`))
    (bind _asaicontroller (cast `AIController` (`self.GetController`)))
    (`DP_AIBaseEvent.SetController` _attackeventref _asaicontroller)
    (`DP_EventHandler.PushEvent` (`self.EnemyEventHandlerRef`) _attackeventref)))

(event `self.Sphere.OnComponentEndOverlap`
  (params (OverlappedComponent :type "PrimitiveComponent Object Reference") (OtherActor :type "Actor Object Reference") (OtherComp :type "PrimitiveComponent Object Reference") (OtherBodyIndex :type Integer))
  (bind _attackeventref (`self.AttackEventRef`))
  (`/Engine/EditorBlueprintResources/StandardMacros.IsValid` _attackeventref
    (:`Is Valid`
      (set `DP_AIAttackEvent.bIsDone` true _attackeventref)
      (set `self.AttackEventRef` null))))

(fn `UserConstructionScript`)