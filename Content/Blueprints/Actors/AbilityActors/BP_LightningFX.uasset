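; BP_LightningFX is an ability effect actor that shapes a lightning effect along a spline through a given set of positions.
; UpdateEffect clears the spline, converts each world position into spline local space and adds it as a linear point, giving straight segments between positions.
; The spline updates once after all points are added, and the construction script is empty.
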(fn `UpdateEffect`
  (params (Positions :type "Array of Vector Structure"))
  (`SplineComponent.ClearSplinePoints` (`self.Spline`) true)
  (for (_array_element _array_index) Positions
    (`SplineComponent.AddPoint` (`self.Spline`) (make `SplinePoint` (`KismetMathLibrary.Conv_IntToDouble` _array_index) (`KismetMathLibrary.InverseTransformLocation` (`SceneComponent.K2_GetComponentToWorld` (`self.Spline`)) _array_element) (0.0 0.0 0.0) (0.0 0.0 0.0) (struct) (1.0 1.0 1.0) "Linear") false))
  (`SplineComponent.UpdateSpline` (`self.Spline`)))

(fn `UserConstructionScript`)