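; BP_ShootingWeaponActor is a shooting weapon ability actor that supplies projectile spawn transforms from five spawn point components.
; On BeginPlay it gathers the five components into a SpawnPoints array.
; The SetProjectileSpawnPoints event clears ProjectileSpawnPoints and refills it with each component's current world transform.
; The file contains no firing or projectile spawning logic.
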(event `self.ReceiveBeginPlay`
  (set `self.SpawnPoints` (`|MakeArray` (`self.SpawnPoint_1`) (`self.SpawnPoint_2`) (`self.SpawnPoint_3`) (`self.SpawnPoint_4`) (`self.SpawnPoint_5`))))

(event `self.SetProjectileSpawnPoints`
  (`KismetArrayLibrary.Array_Clear` (`self.ProjectileSpawnPoints`))
  (for _array_element (`self.SpawnPoints`)
    (`KismetArrayLibrary.Array_Add` (`self.ProjectileSpawnPoints`) (`SceneComponent.K2_GetComponentToWorld` _array_element))))

(fn `UserConstructionScript`)