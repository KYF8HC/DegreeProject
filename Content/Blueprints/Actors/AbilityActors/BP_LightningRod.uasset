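; Lightning rod ability actor that draws a lightning effect between itself and each accepted actor inside its sphere.
; When OnOverlap accepts an entering actor, it spawns a BP_LightningFX and records both in the OverlappingActors array.
; Tick feeds the rod and target locations to each effect so the bolts follow their targets.
; UpdateOverlappingActorsArray destroys a given actor's effect and handles removing its entry; end overlap delegates to OnEndOverlap.
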(event `self.ReceiveTick`
  (params (DeltaSeconds :type "Float (single-precision)"))
  (`self.Update Effects`))

(event `self.Sphere.OnComponentBeginOverlap`
  (params (OverlappedComponent :type "PrimitiveComponent Object Reference") (OtherActor :type "Actor Object Reference") (OtherComp :type "PrimitiveComponent Object Reference") (OtherBodyIndex :type Integer) (bFromSweep :type Boolean) (SweepResult :type "HitResult Structure (by ref)"))
  (bind _returnvalue (`self.OnOverlap` OtherActor))
  (if _returnvalue
    (bind _returnvalue_2 (`|SpawnActorFromClass` "/Game/Blueprints/Actors/AbilityActors/BP_LightningFX.BP_LightningFX_C" (`self.GetTransform`) "AlwaysSpawn" "MultiplyWithRoot" null null))
    (`KismetArrayLibrary.Array_Add` (`self.OverlappingActors`) (make `OverlappingActor` OtherActor true _returnvalue_2))))

(event `self.Sphere.OnComponentEndOverlap`
  (params (OverlappedComponent :type "PrimitiveComponent Object Reference") (OtherActor :type "Actor Object Reference") (OtherComp :type "PrimitiveComponent Object Reference") (OtherBodyIndex :type Integer))
  (`self.OnEndOverlap` OtherActor))

(fn `Update Effects`
  (locals (OverlappingActor :type "OverlappingActor Structure") (InvalidActors :type "Array of OverlappingActor Structure"))
  (bind (_overlappingactorref _biseffectapplied _visualeffectactorref) (break `OverlappingActor` (`local.OverlappingActor`)))
  (for _array_element (`self.OverlappingActors`)
    (set `local.OverlappingActor` _array_element)
    (`KismetArrayLibrary.Array_Clear` (`self.Positions`))
    (`KismetArrayLibrary.Array_Add` (`self.Positions`) (`self.K2_GetActorLocation`))
    (`KismetArrayLibrary.Array_Add` (`self.Positions`) (`self.K2_GetActorLocation` _overlappingactorref))
    (bind _asbp_lightning_fx (cast `/Game/Blueprints/Actors/AbilityActors/BP_LightningFX` _visualeffectactorref))
    (`/Game/Blueprints/Actors/AbilityActors/BP_LightningFX.UpdateEffect` _asbp_lightning_fx (`self.Positions`))))

(fn `UpdateOverlappingActorsArray`
  (params (OtherActor :type "Object Object Reference"))
  (locals (Other :type "Object Object Reference") (ShouldRemove :type Boolean) (Index :type Integer))
  (set `local.Other` OtherActor)
  (for (_array_element _array_index) (`self.OverlappingActors`)
    (bind (_overlappingactorref _biseffectapplied _visualeffectactorref) (break `OverlappingActor` _array_element))
    (bind _output_get (set `local.ShouldRemove` (== _overlappingactorref (`local.Other`))))
    (if _output_get
      (set `local.Index` _array_index)
      (`self.K2_DestroyActor` _visualeffectactorref)))
  (if (`local.ShouldRemove`)
    (`KismetArrayLibrary.Array_Remove` (`self.OverlappingActors`) (`local.Index`))))

(fn `UserConstructionScript`)